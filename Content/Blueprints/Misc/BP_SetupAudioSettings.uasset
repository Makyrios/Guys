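; Blueprint helper that restores the player's saved audio volume settings.
; LoadAudioSettings loads an SV_AudioSettings save from the given slot, stopping if the cast fails, and passes it to ApplySettings.
; ApplySettings sets Master, Interface and Music volumes, each with its own sound mix and class.
; SetSoundClassVolume applies each as a sound mix class override with a short fade, then pushes that mix.
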(fn LoadAudioSettings
  (params (SaveLocation :type String))
  (bind _returnvalue (SaveGame|LoadGamefromSlot SaveLocation))
  (bind _assv_audio_settings (Utilities|Casting|CastToSV_AudioSettings _returnvalue))
  (CallFunction|ApplySettings _assv_audio_settings))

(fn ApplySettings
  (params (AudioSettings :type SV%20Audio%20Settings%20Object%20Reference))
  (CallFunction|SetSoundClassVolume "/Game/Assets/Sounds/Mixes/SCM_Master.SCM_Master" "/Game/Assets/Sounds/Classes/SC_Master.SC_Master" (Variables|/Game/Blueprints/SaveFiles/SV_AudioSettings.SV_AudioSettings_C|GetMasterVolume AudioSettings))
  (CallFunction|SetSoundClassVolume "/Game/Assets/Sounds/Mixes/SCM_Interface.SCM_Interface" "/Game/Assets/Sounds/Classes/SC_Interface.SC_Interface" (Variables|/Game/Blueprints/SaveFiles/SV_AudioSettings.SV_AudioSettings_C|GetInterfaceVolume AudioSettings))
  (CallFunction|SetSoundClassVolume "/Game/Assets/Sounds/Mixes/SCM_Music.SCM_Music" "/Game/Assets/Sounds/Classes/SC_Music.SC_Music" (Variables|/Game/Blueprints/SaveFiles/SV_AudioSettings.SV_AudioSettings_C|GetMusicVolume AudioSettings)))

(fn SetSoundClassVolume
  (params (SoundMix :type Sound%20Mix%20Object%20Reference) (SoundClass :type Sound%20Class%20Object%20Reference) (Volume :type Float%20%28double-precision%29))
  (Audio|SetSoundMixClassOverride 0 SoundMix SoundClass Volume 1.0 0.2 true)
  (Audio|PushSoundMixModifier 0 SoundMix))