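; Gameplay ability that swaps the activating racer's position with the pawn listed just before it in the game state's player progress map.
; After committing, it picks that pawn by key order and ends without effect if the user is first.
; Otherwise it teleport-swaps both actor transforms, applies an instant teleport gameplay effect to both and a slowed-area duration effect to the user.
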(event Ability|EventActivateAbility
  (bind _returnvalue (Ability|GetAvatarActorfromActorInfo))
  (bind _returnvalue_2 (Ability|CommitAbility))
  (if _returnvalue_2
    (bind _asg_race_game_state (Utilities|Casting|CastToG_RaceGameState (Game|GetGameState)))
    (bind _keys (Utilities|Map|Keys (Variables|/Script/Guys.G_RaceGameState|GetPlayerProgressesMap _asg_race_game_state)))
    (if (== (Utilities|Array|FindItem _keys (Ability|GetAvatarActorfromActorInfo)) 0)
      (Ability|EndAbility)
      (else
        (bind _aspawn (Utilities|Casting|CastToPawn (Utilities|Array|Get(acopy) _keys (Math|Integer|Clamp(Integer) (- (Utilities|Array|FindItem _keys (Ability|GetAvatarActorfromActorInfo)) 1) 0 (Utilities|Array|Length _keys)))))
        (Variables|Default|SetTarget _aspawn)
        (Variables|Default|SetTargetTransform (Transformation|GetActorTransform (Variables|Default|GetTarget)))
        (Variables|Default|SetOwnerTransform (Transformation|GetActorTransform _returnvalue))
        (Ability|ApplyGameplayEffectToOwner "/Game/Blueprints/AbilitySystem/Effects/GE_TeleportInstant.GE_TeleportInstant_C")
        (Transformation|SetActorTransform _returnvalue (Variables|Default|GetTargetTransform) false true)
        (Transformation|SetActorTransform (Variables|Default|GetTarget) (Variables|Default|GetOwnerTransform) false true)
        (GameplayEffects|ApplyGameplayEffectToTarget (Ability|TargetData|AbilityTargetDatafromActor (Variables|Default|GetTarget)) "/Game/Blueprints/AbilitySystem/Effects/GE_TeleportInstant.GE_TeleportInstant_C" 1 1)
        (Ability|ApplyGameplayEffectToOwner "/Game/Blueprints/Actors/Areas/SlowedArea/GE_SlowedAreaDuration.GE_SlowedAreaDuration_C")
        (Ability|EndAbility)))))