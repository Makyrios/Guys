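; Gameplay Ability that places a BP_StunArea plate on the ground behind the avatar character.
; On activation it commits the ability, casts the avatar to BP_Character and spawns the area at a fixed offset behind the capsule's forward vector, lowered from the actor's origin, with zero rotation.
; The graph never calls EndAbility, and its OnEndAbility event is an unused stub.
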(event Ability|EventActivateAbility
  (bind _returnvalue (Ability|CommitAbility))
  (if _returnvalue
    (bind _asbp_character (Utilities|Casting|CastToBP_Character (Ability|GetAvatarActorfromActorInfo)))
    (Game|SpawnActorfromClass "/Game/Blueprints/Actors/Areas/StunArea/BP_StunArea.BP_StunArea_C" (Math|Transform|MakeTransform (- (- (Transformation|GetActorLocation _asbp_character) (* (Math|Vector|GetForwardVector (Variables|/Script/Engine.Character|GetCapsuleComponent _asbp_character)) 2e+02)) "0.000000,0.000000,57.000000") (Math|Rotator|Delta(Rotator) "0, 0, 0" "0, 0, 0") "1.000000,1.000000,1.000000") "Undefined" "MultiplyWithRoot" 0 0)))

(event Ability|EventOnEndAbility
  (params (bWasCancelled :type Boolean)))