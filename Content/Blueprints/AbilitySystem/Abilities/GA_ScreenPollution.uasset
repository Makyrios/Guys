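; GA_ScreenPollution is a gameplay ability that applies a temporary Polluted gameplay cue to another character.
; On activation it commits, scans all BP_Character actors and keeps the last one that is not its own avatar as the single target.
; It adds the cue to that target, ends itself after a short delay, and removes the cue when the ability ends.
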(event Ability|EventActivateAbility
  (Ability|CommitAbility)
  (bind _outactors (Actor|GetAllActorsOfClass "/Game/Blueprints/Character/BP_Character.BP_Character_C"))
  (for _array_element _outactors
    (if (!= _array_element (Ability|GetAvatarActorfromActorInfo))
      (Variables|Default|SetTarget _array_element)))
  (GameplayCue|AddGameplayCueOnActor(Looping) (Variables|Default|GetTarget) "(TagName=\"GameplayCue.Polluted\")" (Ability|GameplayCue|MakeGameplayCueParameters 0.0))
  (Utilities|FlowControl|Delay 3.0)
  (Ability|EndAbility))

(event Ability|EventOnEndAbility
  (params (bWasCancelled :type Boolean))
  (GameplayCue|RemoveGameplayCueOnActor(Looping) (Variables|Default|GetTarget) "(TagName=\"GameplayCue.Polluted\")" (Ability|GameplayCue|MakeGameplayCueParameters 0.0)))