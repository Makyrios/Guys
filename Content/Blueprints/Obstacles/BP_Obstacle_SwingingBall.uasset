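; Swinging ball obstacle that knocks BP_Character away on contact.
; When its Sphere begins overlapping a character, it toggles that character's physical animation and launches it hard along the direction from the sphere's center to the character.
; When the character stops overlapping the actor, a short delay runs before physics simulation on its mesh is switched off.
; The graph contains no swing logic, only this hit response.
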(event Custom|OnComponentBeginOverlap_Event
  (params (OverlappedComponent :type Primitive%20Component%20Object%20Reference) (OtherActor :type Actor%20Object%20Reference) (OtherComp :type Primitive%20Component%20Object%20Reference) (OtherBodyIndex :type Integer) (bFromSweep :type Boolean) (SweepResult :type Hit%20Result%20Structure%20%28by%20ref%29))
  (bind _asbp_character (Utilities|Casting|CastToBP_Character OtherActor))
  (Class|GPhysicalAnimComponent|TogglePhysicalAnimation (Variables|/Script/Guys.G_Character|GetPhysicalAnimComponent _asbp_character) 1.0)
  (Character|LaunchCharacter _asbp_character (* (Math|Vector|Normalize (- (Transformation|GetActorLocation _asbp_character) (Transformation|GetWorldLocation (Variables|Default|GetSphere)))) 1e+04) false false))

(event EventBeginPlay
  (Collision|AssignOnComponentBeginOverlap (Variables|Default|GetSphere) (delegate Custom|OnComponentBeginOverlap_Event)))

(event EventTick
  (params (DeltaSeconds :type Float%20%28single-precision%29)))

(event Collision|EventActorEndOverlap
  (params (OtherActor :type Actor%20Object%20Reference))
  (bind _asbp_character (Utilities|Casting|CastToBP_Character OtherActor))
  (Utilities|FlowControl|Delay 1.0)
  (Physics|SetSimulatePhysics (Variables|/Script/Engine.Character|GetMesh _asbp_character) false))

(fn ConstructionScript)